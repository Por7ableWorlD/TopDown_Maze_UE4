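; Player-controlled tank that moves in four directions and fires missiles.
; MoveForward and MoveRight input first snap the actor to the matching heading, stored in DirectionOfRotation, then step it along local Y by a fixed, swept offset per input event.
; Left click spawns a BP_Missile at SpawnPlaceMissile, and three helper functions set its Direction from that heading.
; The forward heading has no helper, leaving the missile's Direction unchanged.
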(event `InputAxis|MoveForward`
  (params (AxisValue :type "Float (single-precision)"))
  ;[1 1 1] Forward/backward movement
  (if (> AxisValue 0.0)
    (if (!= (`self.DirectionOfRotation`) 1)
      (`self.K2_SetActorRotation` (struct :`Yaw` 90.0))
      (set `self.DirectionOfRotation` 1)
      (else
        (`self.K2_AddActorLocalOffset` (0.0 12.0 0.0) true)))))

(event `InputAxis|MoveForward`
  (params (AxisValue :type "Float (single-precision)"))
  ;[1 1 1] Forward/backward movement
  (if (< AxisValue 0.0)
    (if (!= (`self.DirectionOfRotation`) 0)
      (`self.K2_SetActorRotation` (struct :`Yaw` -90.0))
      (set `self.DirectionOfRotation` 0)
      (else
        (`self.K2_AddActorLocalOffset` (0.0 12.0 0.0) true)))))

(event `InputAxis|MoveRight`
  (params (AxisValue :type "Float (single-precision)"))
  ;[1 1 1] Right/left movement
  (if (> AxisValue 0.0)
    (if (!= (`self.DirectionOfRotation`) 3)
      (`self.K2_SetActorRotation` (struct :`Yaw` 180.0))
      (set `self.DirectionOfRotation` 3)
      (else
        (`self.K2_AddActorLocalOffset` (0.0 12.0 0.0) true)))))

(event `InputAxis|MoveRight`
  (params (AxisValue :type "Float (single-precision)"))
  ;[1 1 1] Right/left movement
  (if (< AxisValue 0.0)
    (if (!= (`self.DirectionOfRotation`) 2)
      (`self.K2_SetActorRotation` (struct))
      (set `self.DirectionOfRotation` 2)
      (else
        (`self.K2_AddActorLocalOffset` (0.0 12.0 0.0) true)))))

(event `Key|LeftMouseButton`
  (params (Key :type "Key Structure"))
  ;[1 1 1] Shooting
  (:`Pressed`
    (bind _returnvalue (`|SpawnActorFromClass` "/Game/GameLogic/Blueprints_Game/BP_Missile.BP_Missile_C" (`KismetMathLibrary.Conv_VectorToTransform` (`SceneComponent.K2_GetComponentLocation` (`self.SpawnPlace_Missile`))) "AlwaysSpawn" "OverrideRootScale" null null))
    (`self.LeftShotDirection` _returnvalue)
    (`self.RigthShotDirection` _returnvalue)
    (`self.BackShotDirection` _returnvalue)))

(fn `BackShotDirection`
  (params (Missile :type "/Game/GameLogic/Blueprints_Game/BP_Missile Object Reference"))
  (if (== (`self.DirectionOfRotation`) 0)
    (set `/Game/GameLogic/Blueprints_Game/BP_Missile.Direction` (100.0 0.0 0.0) Missile)))

(fn `LeftShotDirection`
  (params (Missile :type "/Game/GameLogic/Blueprints_Game/BP_Missile Object Reference"))
  (if (== (`self.DirectionOfRotation`) 2)
    (set `/Game/GameLogic/Blueprints_Game/BP_Missile.Direction` (0.0 100.0 0.0) Missile)))

(fn `RigthShotDirection`
  (params (Missile :type "/Game/GameLogic/Blueprints_Game/BP_Missile Object Reference"))
  (if (== (`self.DirectionOfRotation`) 3)
    (set `/Game/GameLogic/Blueprints_Game/BP_Missile.Direction` (0.0 -100.0 0.0) Missile)))

(fn `UserConstructionScript`)